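; Function library for the card game toolkit that computes a widget transform for each card in a hand layout.
; Fanned and Horizontal derive position, scale and optional tilt from the card's signed distance to the center, with a quadratic RadiusOffset arc and FlyInDirection mirroring.
; Fanned centers on the current card count and can widen spacing for smaller hands.
; Horizontal centers on maximum hand size with fixed spacing, leaving its dynamic-spacing calculation unconnected.
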(fn `Fanned`
  (params (CardWidgetReference :type "Widget Object Reference") (CardLoopIndex :type Integer) (CardsInHand :type Integer) (MaxCardsInHand :type Integer) (`Screen Resolution` :type "Vector2D Structure") (`Card Size` :type "Vector2D Structure") (FlyInDirection :type Boolean) (RotateCardsToOffset :type Boolean) (CardOffset :type "Float (double-precision)") (RotationDistanceScaleFactor :type "Float (double-precision)") (RadiusOffset :type "Float (double-precision)") (`CardSpacing(Min)` :type "Float (double-precision)") (DynamicSpacing :type Boolean) (DynamicSpacingMaxOffset :type "Float (double-precision)") (ScreenOffsetX :type "Float (double-precision)") (ScreenOffsetY :type "Float (double-precision)") (ViewportScale :type "Float (double-precision)") (CardScale :type "Float (double-precision)"))
  (returns (GoalTransform :type "WidgetTransform Structure"))
  (bind _returnvalue (`KismetMathLibrary.Conv_IntToDouble` CardLoopIndex))
  (bind _returnvalue_2 (+ (/ (`KismetMathLibrary.Conv_IntToDouble` (- CardsInHand 1)) 2.0) CardOffset))
  (bind _returnvalue_3 (- _returnvalue _returnvalue_2))
  (bind _returnvalue_4 (* _returnvalue_3 (* RotationDistanceScaleFactor 20.0)))
  (bind _returnvalue_5 (* _returnvalue_3 (select `bool` DynamicSpacing :`false` `CardSpacing(Min)` :`true` (`KismetMathLibrary.FClamp` (`KismetMathLibrary.Lerp` DynamicSpacingMaxOffset `CardSpacing(Min)` (/ (`KismetMathLibrary.Conv_IntToDouble` CardsInHand) (`KismetMathLibrary.Conv_IntToDouble` MaxCardsInHand))) `CardSpacing(Min)` DynamicSpacingMaxOffset))))
  (bind _returnvalue_6 (* _returnvalue_4 -1.0))
  (return (make `WidgetTransform` :`Translation` (`KismetMathLibrary.MakeVector2D` (+ ScreenOffsetX (* (select `bool` FlyInDirection :`false` (* _returnvalue_5 -1.0) :`true` _returnvalue_5) CardScale)) (* (- (* (* _returnvalue_3 (* _returnvalue_5 RadiusOffset)) -1.0) ScreenOffsetY) CardScale)) :`Scale` (`KismetMathLibrary.MakeVector2D` CardScale CardScale) :`Angle` (* (select `bool` RotateCardsToOffset :`true` (select `bool` (>= _returnvalue _returnvalue_2) :`false` (select `bool` FlyInDirection :`false` _returnvalue_4 :`true` _returnvalue_6) :`true` (select `bool` FlyInDirection :`false` _returnvalue_4 :`true` _returnvalue_6))) -1.0))))

(fn `Horizontal`
  (params (CardWidgetReference :type "Widget Object Reference") (CardLoopIndex :type Integer) (CardsInHand :type Integer) (MaxCardInHand :type Integer) (ScreenResolution :type "Vector2D Structure") (`Card Size` :type "Vector2D Structure") (`Fly in Direction` :type Boolean) (RotateCardsToOffset :type Boolean) (RadiusOffset :type "Float (double-precision)") (RotationDistanceScaleFactor :type "Float (double-precision)") (CardSpacing :type "Float (double-precision)") (DynamicSpacing :type Boolean) (CardSpacingMax :type "Float (double-precision)") (ScreenOffsetX :type "Float (double-precision)") (ScreenOffsetY :type "Float (double-precision)") (CardScale :type "Float (double-precision)") (ViewportScale :type "Float (double-precision)") (CardOffset :type "Float (double-precision)"))
  (returns (GoalTransform :type "WidgetTransform Structure"))
  (bind _returnvalue (`KismetMathLibrary.Conv_IntToDouble` CardLoopIndex))
  (bind _returnvalue_2 (- _returnvalue (+ (/ (`KismetMathLibrary.Conv_IntToDouble` (- MaxCardInHand 1)) 2.0) CardOffset)))
  (bind _returnvalue_3 (* _returnvalue_2 (* RotationDistanceScaleFactor 20.0)))
  (bind _returnvalue_4 (* _returnvalue_2 CardSpacing))
  (bind _returnvalue_5 (* _returnvalue_3 -1.0))
  (bind _returnvalue_6 (* (- _returnvalue_4 0.0) CardScale))
  (return (make `WidgetTransform` (`KismetMathLibrary.MakeVector2D` (+ (select `bool` `Fly in Direction` :`false` (* _returnvalue_6 -1.0) :`true` _returnvalue_6) ScreenOffsetX) (* (- (+ (* (* _returnvalue_2 (* _returnvalue_4 RadiusOffset)) -1.0) 1.0) ScreenOffsetY) CardScale)) (`KismetMathLibrary.MakeVector2D` CardScale CardScale) (0.0 0.0) (* (select `bool` RotateCardsToOffset :`true` (select `bool` (>= _returnvalue (`KismetMathLibrary.Conv_IntToDouble` CardsInHand)) :`false` (select `bool` `Fly in Direction` :`false` _returnvalue_3 :`true` _returnvalue_5) :`true` (select `bool` `Fly in Direction` :`false` _returnvalue_3 :`true` _returnvalue_5))) -1.0))))